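; MyHud is a HUD Blueprint that draws a frame rate counter on screen.
; Tick derives FPS from the inverse of delta time and picks a red text colour below a low threshold, blue otherwise.
; DrawHUD renders the labelled value with that colour in a set font.
; A disconnected debug print for bad FPS remains in the graph and never runs.
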(event EventBeginPlay)

(event EventActorBeginOverlap
  (params (OtherActor :type Actor%20Object%20Reference)))

(event EventTick
  (params (DeltaSeconds :type Float%20%28single-precision%29))
  (bind _output_get (Variables|Default|SetFPS (Math|Float|Floor (/ 1.0 DeltaSeconds))))
  (if (< _output_get 20)
    (Variables|Default|SetFPSColour "(R=0.600000,G=0.005457,B=0.000000,A=1.000000)")
    (else
      (Variables|Default|SetFPSColour "(R=0.119603,G=0.421118,B=0.605000,A=1.000000)"))))

(event EventDrawHUD
  (params (SizeX :type Integer) (SizeY :type Integer))
  (HUD|DrawText (Utilities|String|Append (Utilities|String|MakeLiteralString "FPS ") (Utilities|String|ToString(Integer) (Variables|Default|GetFPS))) (Variables|Default|GetFPSColour) 0.0 0.0 "/Game/Blueprints/NewFont.NewFont" 1.0 false))

(fn ConstructionScript)