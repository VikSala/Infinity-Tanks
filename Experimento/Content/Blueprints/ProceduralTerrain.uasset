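; Procedural terrain actor that tiles static mesh sections around player zero's pawn, starting with a flat piece and a randomly chosen biome at BeginPlay.
; While the pawn moves, Tick walks a snapped grid, line-tracing each cell and filling empty ones with rotated, optionally random and Z-scaled pieces.
; Index-zero pieces can receive spawned Blueprint actors and instanced detail meshes.
; Saved section positions drive distance-based removal of old sections and their detail instances.
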(event EventBeginPlay
  (bind _biom_types (Variables|generation|GetBiom_Types))
  (Utilities|SectionPlacement 0 0 false ; place one flat section under where the player starts
    (:NewParam1
      ;[1 1 1] Random Between Set Bioms
      (Variables|SpawnerMemory|SetBiom (Utilities|Array|Get(acopy) _biom_types (Math|Random|RandomIntegerinRange 0 (Utilities|Array|LastIndex _biom_types))))
      ;[1 1 1] create instanced detail mesh
      (if (Variables|DetailMesh|GetDetailMeshEnabled)
        (bind _returnvalue (AddComponent|AddInstancedStaticMeshComponent false))
        (Rendering|SetCastShadow _returnvalue (Variables|DetailMesh|GetDetailMeshCastShadows))
        (Components|StaticMesh|SetStaticMesh _returnvalue (Variables|DetailMesh|GetDetailMesh))
        (Variables|DetailMesh|SetDetailMeshInstance _returnvalue)))))

(event EventTick
  (params (DeltaSeconds :type Float%20%28single-precision%29))
  (if (> (Math|Vector|VectorLength (Transformation|GetVelocity (Pawn|GetControlledPawn (Game|GetPlayerController 0)))) 0.0)
    (bind (_returnvalue _returnvalue2) (|GridMaker) ; makes a grid and fires an event for each grid section with a x and y value.
      (:LoopBody
        (Utilities|SectionPlacement _returnvalue2 _returnvalue (Variables|generation|GetRandomPieces) ; where the mesh sections are acctualy spawned
          (:NewParam1
            (|DeleteUnNeededMapSections) ; DeleteUnNeededMapSections based on distance
          ))))))

(fn ConstructionScript)